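; Health component for an actor, built around zombies, that handles damage, hit feedback and death.
; The damage event subtracts from Health and, once it drops below zero, notifies the spawn system if one is flagged and destroys the owner, guarded by IsDying.
; Surviving hits on a BP_Zombie owner briefly pulse the OnHit material parameter.
; The OnDeadHandlerEvent function is an empty stub.
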(event `OnTakeDamage_Event`
  (params (Damage :type Integer))
  ;[1 1 1] Health System
  (bind _output_get (set `self.Health` (- (`self.Health`) Damage)))
  (if (< _output_get 0)
    (if (not (`self.isDying`))
      (set `self.isDying` true)
      (if (`self.hasSpawn`)
        (`/Game/Blueprint/Bp_SpawnSystem.OnZombieDied` (`self.SpawnSystem`)))
      (`Actor.K2_DestroyActor` (`self.GetOwner`)))
    (else
      (bind _asbp_zombie (cast `/Game/Blueprint/BP_Zombie` (`self.GetOwner`)))
      (bind _mat (`/Game/Blueprint/BP_Zombie.Mat` _asbp_zombie))
      (`MaterialInstanceDynamic.SetScalarParameterValue` _mat "OnHit" 1.0)
      (`KismetSystemLibrary.Delay` 0.5)
      (`MaterialInstanceDynamic.SetScalarParameterValue` _mat "OnHit" 0.0))))

(fn `OnDeadHandler_Event`)