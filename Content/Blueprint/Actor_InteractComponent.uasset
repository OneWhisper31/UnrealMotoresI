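; Actor interact component that supplies shared events for interactable objects the first-person character can use at a cost.
; Overlap shows the price on the character's price UI and stores the object as its current overlap target.
; Ending overlap hides the price and clears that target.
; Interaction either calls the player's win handler, passing a final-level flag, or destroys the interacted actor.
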(event `OnInteract_Event`
  (params (OnInteractWin :type Boolean) (_self :type "Actor Object Reference") (IsFinalLevel :type Boolean))
  (if OnInteractWin
    (bind _asbp_first_person_character (cast `/Game/FirstPerson/Blueprints/BP_FirstPersonCharacter` (`GameplayStatics.GetPlayerCharacter` 0)))
    (`/Game/FirstPerson/Blueprints/BP_FirstPersonCharacter.OnWin` _asbp_first_person_character IsFinalLevel)
    (else
      (`Actor.K2_DestroyActor` _self))))

(event `OnOverlap_Event`
  (params (other :type "Actor Object Reference") (_self :type "Actor Object Reference") (cost :type Integer))
  (bind _asbp_first_person_character (cast `/Game/FirstPerson/Blueprints/BP_FirstPersonCharacter` other))
  (`/Game/UI/WB_Interact.UpdateInteractPrice` (`/Game/FirstPerson/Blueprints/BP_FirstPersonCharacter.InteractPriceReference` _asbp_first_person_character) cost)
  (bind _asbp_interatable_object (cast `/Game/Blueprint/BP_InteratableObject` _self))
  (set `/Game/FirstPerson/Blueprints/BP_FirstPersonCharacter.OnOverlap` _asbp_interatable_object _asbp_first_person_character))

(event `StopOverlap_Event`
  (params (other :type "Actor Object Reference"))
  (bind _asbp_first_person_character (cast `/Game/FirstPerson/Blueprints/BP_FirstPersonCharacter` other))
  (`/Game/UI/WB_Interact.HidePrice` (`/Game/FirstPerson/Blueprints/BP_FirstPersonCharacter.InteractPriceReference` _asbp_first_person_character))
  (set `/Game/FirstPerson/Blueprints/BP_FirstPersonCharacter.OnOverlap` null _asbp_first_person_character))