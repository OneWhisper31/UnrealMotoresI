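; Interactable object Blueprint that the first-person player can use, with a cost shown while in range.
; Collider overlap shows the cost on the character's interact price display and registers the object as its OnOverlap target, clearing both on exit.
; OnInteract either triggers the player's OnWin when the win flag is set, or destroys the object.
; The cost is only displayed here, with no payment check in this asset.
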(event `OnInteract`
  (if (`self.OnInteractWin`)
    (bind _asbp_first_person_character (cast `/Game/FirstPerson/Blueprints/BP_FirstPersonCharacter` (`GameplayStatics.GetPlayerCharacter` 0)))
    (`/Game/FirstPerson/Blueprints/BP_FirstPersonCharacter.OnWin` _asbp_first_person_character)
    (else
      (`self.K2_DestroyActor`))))

(event `self.Collider.OnComponentBeginOverlap`
  (params (OverlappedComponent :type "PrimitiveComponent Object Reference") (OtherActor :type "Actor Object Reference") (OtherComp :type "PrimitiveComponent Object Reference") (OtherBodyIndex :type Integer) (bFromSweep :type Boolean) (SweepResult :type "HitResult Structure (by ref)"))
  (bind _asbp_first_person_character (cast `/Game/FirstPerson/Blueprints/BP_FirstPersonCharacter` OtherActor))
  (`/Game/UI/WB_Interact.UpdateInteractPrice` (`/Game/FirstPerson/Blueprints/BP_FirstPersonCharacter.InteractPriceReference` _asbp_first_person_character) (`self.Cost`))
  (set `/Game/FirstPerson/Blueprints/BP_FirstPersonCharacter.OnOverlap` self _asbp_first_person_character))

(event `self.Collider.OnComponentEndOverlap`
  (params (OverlappedComponent :type "PrimitiveComponent Object Reference") (OtherActor :type "Actor Object Reference") (OtherComp :type "PrimitiveComponent Object Reference") (OtherBodyIndex :type Integer))
  (bind _asbp_first_person_character (cast `/Game/FirstPerson/Blueprints/BP_FirstPersonCharacter` OtherActor))
  (`/Game/UI/WB_Interact.HidePrice` (`/Game/FirstPerson/Blueprints/BP_FirstPersonCharacter.InteractPriceReference` _asbp_first_person_character))
  (set `/Game/FirstPerson/Blueprints/BP_FirstPersonCharacter.OnOverlap` null _asbp_first_person_character))

(fn `UserConstructionScript`)