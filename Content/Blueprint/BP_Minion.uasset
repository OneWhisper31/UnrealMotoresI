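; BP_Minion is an AI enemy that feeds player awareness and proximity to its Blackboard.
; Pawn sensing flags the player as seen, and Tick checks a short distance threshold.
; On range changes, gated by OnAnimEnded, it updates the range key, sets the seen key and stops movement.
; Damage forwards to ActorHealthComponent, and BeginPlay puts an "OnHit" dynamic material on the mesh.
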(event `self.ReceiveBeginPlay`
  (bind _returnvalue (`KismetMaterialLibrary.CreateDynamicMaterialInstance` "/Game/Models/Materials/material_002.material_002" "OnHit"))
  (bind _output_get (set `self.Mat` _returnvalue))
  (`PrimitiveComponent.SetMaterial` (`self.Mesh`) 3 _output_get))

(event `self.ReceiveTick`
  (params (DeltaSeconds :type "Float (single-precision)"))
  (bind _returnvalue (`AIBlueprintHelperLibrary.GetBlackboard` (`AIBlueprintHelperLibrary.GetAIController` self)))
  (bind _returnvalue_2 (<= (`KismetMathLibrary.Vector_Distance` (`self.K2_GetActorLocation`) (`self.K2_GetActorLocation` (`GameplayStatics.GetPlayerCharacter` 0))) 200.0))
  ;[1 1 1] IsOnRange
  (if (!= _returnvalue_2 (`self.isOnRange`))
    (if (`self.onAnimEnded`)
      (bind _output_get (set `self.isOnRange` _returnvalue_2))
      (`BlackboardComponent.SetValueAsBool` _returnvalue "isOnRange" _output_get)
      (`BlackboardComponent.SetValueAsBool` _returnvalue "hasSeenPlayer?" true)
      (`Controller.StopMovement` (`AIBlueprintHelperLibrary.GetAIController` self)))))

(event `self.PawnSensing.OnSeePawn`
  (params (Pawn :type "Pawn Object Reference"))
  ;[1 1 1] hasSeenPlayer?
  (cast `/Game/FirstPerson/Blueprints/BP_FirstPersonCharacter` Pawn)
  (`BlackboardComponent.SetValueAsBool` (`AIBlueprintHelperLibrary.GetBlackboard` (`AIBlueprintHelperLibrary.GetAIController` self)) "hasSeenPlayer?" true))

(event `OnTakeDamage_Event`
  (params (Damage :type Integer))
  (`/Game/Blueprint/Actor_HealthComponent.OnTakeDamage_Event` (`self.Actor_HealthComponent`) Damage))

(fn `UserConstructionScript`)