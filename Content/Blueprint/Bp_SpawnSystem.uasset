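; Zombie spawner actor that keeps the enemy population topped up around a configured maximum.
; BeginPlay caches two waypoint sets from child component locations and registers the spawner with the first-person player character.
; Tick uses Delay nodes to throttle spawning at random waypoints; OnOpen shortens the delay and adds the second set as a random option.
; Each zombie receives a spawner reference, and OnZombieDied decrements the count.
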(event `self.ReceiveBeginPlay`
  ;[1 1 1] Initialize Waypoints
  (for _array_element (`SceneComponent.GetChildrenComponents` (`self.Waypoint`) false)
    (`KismetArrayLibrary.Array_Add` (`self.waypoints`) (`SceneComponent.K2_GetComponentLocation` _array_element)))
  (for _array_element_2 (`SceneComponent.GetChildrenComponents` (`self.Waypoint2`) false)
    (`KismetArrayLibrary.Array_Add` (`self.waypoints2`) (`SceneComponent.K2_GetComponentLocation` _array_element_2)))
  (`KismetSystemLibrary.DelayUntilNextTick`)
  (bind _asbp_first_person_character (cast `/Game/FirstPerson/Blueprints/BP_FirstPersonCharacter` (`GameplayStatics.GetPlayerCharacter` 0)))
  (set `/Game/FirstPerson/Blueprints/BP_FirstPersonCharacter.BP_SpawnSytem` self _asbp_first_person_character))

(event `self.ReceiveTick`
  (params (DeltaSeconds :type "Float (single-precision)"))
  ;[1 1 1] Update
  (if (<= (`self.enemyCount`) (`self.maxenemies`))
    (if (`self.onOpen`)
      (`KismetSystemLibrary.Delay` 1.0)
      (else
        (`KismetSystemLibrary.Delay` 2.0)))
    (set `self.enemyCount` (+ (`self.enemyCount`) 1))
    (if (`self.onOpen`)
      (if (<= (`KismetMathLibrary.RandomInteger` 10) 5)
        (bind _zombie (`self.SpawnZombie` (`self.waypoints2`)))
        (set `/Game/Blueprint/BP_Zombie.spawnSystem` self _zombie)
        (else
          (bind _zombie_2 (`self.SpawnZombie` (`self.waypoints`) :!label _label))
          (set `/Game/Blueprint/BP_Zombie.spawnSystem` self _zombie_2)))
      (else
        (goto _label)))))

(event `OnZombieDied`
  ;[1 1 1] OnZombieDied
  (set `self.enemyCount` (- (`self.enemyCount`) 1)))

(fn `UserConstructionScript`)