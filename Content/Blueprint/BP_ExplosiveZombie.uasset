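; BP_ExplosiveZombie is the explosive zombie enemy, feeding AI blackboard state and taking damage through a health component.
; BeginPlay loads health from the ZombieTable data table and puts a dynamic "OnHit" material on the mesh.
; Tick sets the in-range key from distance to the player, and pawn sensing flags when the player is seen.
; Damage events forward to ActorHealthComponent; no explosion logic appears in these graphs.
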(event `self.ReceiveBeginPlay`
  (bind _returnvalue (`KismetMaterialLibrary.CreateDynamicMaterialInstance` "/Game/Models/Materials/material_002.material_002" "OnHit"))
  (bind _output_get (set `self.Mat` _returnvalue))
  (`PrimitiveComponent.SetMaterial` (`self.Mesh`) 3 _output_get)
  (bind _returnvalue_2 (`|GetDataTableRow` "/Game/DataValue/ZombieTable.ZombieTable" "ZombieExplosive")
    (:`then`
      (set `/Game/Blueprint/Actor_HealthComponent.Health` (`.Health_10_4A201E2D4348A9CE2C5CBAAA64F0B12D` (break `/Game/DataValue/DataValueRowZombie` _returnvalue_2)) (`self.Actor_HealthComponent`)))))

(event `self.ReceiveTick`
  (params (DeltaSeconds :type "Float (single-precision)"))
  ;[1 1 1] IsOnRange
  (`BlackboardComponent.SetValueAsBool` (`AIBlueprintHelperLibrary.GetBlackboard` (`AIBlueprintHelperLibrary.GetAIController` self)) "isOnRange" (<= (`KismetMathLibrary.Vector_Distance` (`self.K2_GetActorLocation`) (`self.K2_GetActorLocation` (`GameplayStatics.GetPlayerCharacter` 0))) 100.0)))

(event `self.PawnSensing.OnSeePawn`
  (params (Pawn :type "Pawn Object Reference"))
  ;[1 1 1] hasSeenPlayer?
  (cast `/Game/FirstPerson/Blueprints/BP_FirstPersonCharacter` Pawn)
  (`BlackboardComponent.SetValueAsBool` (`AIBlueprintHelperLibrary.GetBlackboard` (`AIBlueprintHelperLibrary.GetAIController` self)) "hasSeenPlayer?" true))

(event `OnTakeDamage_Event`
  (params (Damage :type Integer))
  (`/Game/Blueprint/Actor_HealthComponent.OnTakeDamage_Event` (`self.Actor_HealthComponent`) Damage))

(fn `UserConstructionScript`)