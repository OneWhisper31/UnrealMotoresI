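; Zombie enemy that chases the player and attacks in melee, with incoming damage forwarded to its health component.
; Tick reissues AI MoveTo toward the player whenever it is not attacking; arrival plays an attack montage.
; Halfway through the montage, a distance check decides whether the player takes damage, and a miss ends the attack immediately.
; BeginPlay creates and stores an "OnHit" dynamic material on the mesh, unused in these graphs.
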(event `OnTakeDamage`
  (params (damage :type Integer))
  ;[1 1 1] Health System
  (`/Game/Blueprint/Actor_HealthComponent.OnTakeDamage_Event` (`self.Actor_HealthComponent`) damage))

(event `self.ReceiveBeginPlay`
  (bind _returnvalue (`KismetMaterialLibrary.CreateDynamicMaterialInstance` "/Game/Models/Materials/material_002.material_002" "OnHit"))
  (set `self.Mat` _returnvalue)
  (`PrimitiveComponent.SetMaterial` (`self.Mesh`) 3 _returnvalue))

(event `self.ReceiveTick`
  (params (DeltaSeconds :type "Float (single-precision)"))
  (bind _returnvalue (`GameplayStatics.GetPlayerCharacter` 0))
  (if (not (`self.isAttacking`))
    (`|AIMoveTo` self (0.0 0.0 0.0) _returnvalue 70.0
      (:`OnSuccess`
        (set `self.isAttacking` true)
        (bind _returnvalue_2 (`self.PlayAnimMontage` "/Game/Animation/Zombie/Zombie_AttackMontage.Zombie_AttackMontage"))
        (bind _returnvalue_3 (/ _returnvalue_2 2.0))
        (`KismetSystemLibrary.Delay` _returnvalue_3)
        (if (< (`KismetMathLibrary.Vector_Distance` (`self.K2_GetActorLocation` _returnvalue) (`self.K2_GetActorLocation` self)) 200.0)
          (bind _asbp_first_person_character (cast `/Game/FirstPerson/Blueprints/BP_FirstPersonCharacter` _returnvalue))
          (`/Game/FirstPerson/Blueprints/BP_FirstPersonCharacter.OnTakeDamage` _asbp_first_person_character (`self.Damage`))
          (`KismetSystemLibrary.Delay` _returnvalue_3))
        (set `self.isAttacking` false)))))

(fn `UserConstructionScript`)