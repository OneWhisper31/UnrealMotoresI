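; BP_SaveHandler is an actor that persists level-specific player positions in a BP_SaveGame slot.
; BeginPlay restores the player's transform by LevelIndex and Points from the save, or creates a save with Points zeroed on the character.
; A delayed Tick autosaves roughly every five seconds, storing the handler's own transform rather than the player's.
; Each autosave copies saved Points onto BP_FirstPersonCharacter, never the reverse.
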(event `self.ReceiveBeginPlay`
  (bind _returnvalue (`self.GetTransform`))
  (bind _returnvalue_2 (`GameplayStatics.GetPlayerCharacter` 0))
  (bind _returnvalue_3 (`GameplayStatics.DoesSaveGameExist` "save"))
  (if _returnvalue_3
    (bind _returnvalue_4 (`GameplayStatics.LoadGameFromSlot` "save"))
    (bind _asbp_save_game (cast `/Game/Blueprint/BP_SaveGame` _returnvalue_4))
    (bind _output_get (set `self.BP_SaveGame` _asbp_save_game))
    (switch `int` (`/Game/Blueprint/BP_SaveGame.LevelIndex` _asbp_save_game)
      (:`Default`
        (`self.K2_SetActorTransform` _returnvalue_2 (`/Game/Blueprint/BP_SaveGame.playerPosLevel1` _output_get) false false :!label _label))
      (:`0`
        (goto _label))
      (:`1`
        (goto _label))
      (:`2`
        (`self.K2_SetActorTransform` _returnvalue_2 (`/Game/Blueprint/BP_SaveGame.playerPosLevel2` _output_get) false false))
      (:`3`
        (`self.K2_SetActorTransform` _returnvalue_2 (`/Game/Blueprint/BP_SaveGame.playerPosLevel3` _output_get) false false)))
    (bind _asbp_first_person_character (cast `/Game/FirstPerson/Blueprints/BP_FirstPersonCharacter` _returnvalue_2))
    (set `/Game/FirstPerson/Blueprints/BP_FirstPersonCharacter.Points` (`/Game/Blueprint/BP_SaveGame.Points` _output_get) _asbp_first_person_character)
    (else
      (bind _returnvalue_5 (`GameplayStatics.CreateSaveGameObject` "/Game/Blueprint/BP_SaveGame.BP_SaveGame_C"))
      (bind _output_get_2 (set `self.BP_SaveGame` _returnvalue_5))
      (switch `int` (`/Game/Blueprint/BP_SaveGame.LevelIndex` _output_get_2)
        (:`Default`
          (set `/Game/Blueprint/BP_SaveGame.playerPosLevel1` _returnvalue _output_get_2 :!label _label_2))
        (:`0`
          (goto _label_2))
        (:`1`
          (goto _label_2))
        (:`2`
          (set `/Game/Blueprint/BP_SaveGame.playerPosLevel2` _returnvalue _output_get_2))
        (:`3`
          (set `/Game/Blueprint/BP_SaveGame.playerPosLevel3` _returnvalue _output_get_2)))
      (`GameplayStatics.SaveGameToSlot` _output_get_2 "save")
      (bind _asbp_first_person_character_2 (cast `/Game/FirstPerson/Blueprints/BP_FirstPersonCharacter` _returnvalue_2))
      (set `/Game/FirstPerson/Blueprints/BP_FirstPersonCharacter.Points` 0 _asbp_first_person_character_2)
      (`KismetSystemLibrary.PrintString` "crated"))))

(event `self.ReceiveTick`
  (params (DeltaSeconds :type "Float (single-precision)"))
  (bind _returnvalue (`self.GetTransform`))
  (bind _bp_savegame (`self.BP_SaveGame`))
  (`KismetSystemLibrary.Delay` 5.0)
  (bind _returnvalue_2 (`GameplayStatics.DoesSaveGameExist` "save"))
  (if _returnvalue_2
    (switch `int` (`/Game/Blueprint/BP_SaveGame.LevelIndex` _bp_savegame)
      (:`Default`
        (set `/Game/Blueprint/BP_SaveGame.playerPosLevel1` _returnvalue _bp_savegame :!label _label_3))
      (:`0`
        (goto _label_3))
      (:`1`
        (goto _label_3))
      (:`2`
        (set `/Game/Blueprint/BP_SaveGame.playerPosLevel2` _returnvalue _bp_savegame))
      (:`3`
        (set `/Game/Blueprint/BP_SaveGame.playerPosLevel3` _returnvalue _bp_savegame)))
    (`GameplayStatics.SaveGameToSlot` _bp_savegame "save")
    (bind _asbp_first_person_character (cast `/Game/FirstPerson/Blueprints/BP_FirstPersonCharacter` (`GameplayStatics.GetPlayerCharacter` 0)))
    (set `/Game/FirstPerson/Blueprints/BP_FirstPersonCharacter.Points` (`/Game/Blueprint/BP_SaveGame.Points` _bp_savegame) _asbp_first_person_character)
    (`KismetSystemLibrary.PrintString` "Saved")))

(fn `UserConstructionScript`)